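; BP_PlayerCharactor02 is a side-scrolling player character with a Paper2D flipbook, HP and Enhanced Input controls.
; BeginPlay adds the input mapping and base UI; movement runs along X behind a CanMove gate, flipping rotation to face travel.
; Jump input swaps jump and walk flipbooks, and damage subtracts from HP.
; Interact only looks up BP_NPC_Guide, as its range check and interaction logic are disconnected.
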(event `SetUIBase`
  (bind _returnvalue (`|CreateWidget` "/Game/MyProject/C03/UI_Base.UI_Base_C"))
  (`UserWidget.AddToViewport` _returnvalue 0))

(event `self.ReceiveBeginPlay`
  (`EnhancedInputSubsystemInterface.AddMappingContext` (pcsubsystem `EnhancedInputLocalPlayerSubsystem` (`GameplayStatics.GetPlayerController` 0)) "/Game/MyProject/C03/Input/IMC_Player01.IMC_Player01" 0 (struct))
  (`self.SetUIBase`))

(event `EnhancedInput|/Game/MyProject/C03/Input/IA_Move01`
  (params (ActionValue :type "Vector2D Structure") (ElapsedSeconds :type "Float (double-precision)") (TriggeredSeconds :type "Float (double-precision)") (InputAction :type "InputAction Object Reference" :default "/Game/MyProject/C03/Input/IA_Move01.IA_Move01"))
  (bind _x (`KismetMathLibrary.BreakVector2D` ActionValue))
  (:`Triggered`
    (if (`self.CanMove`)
      (if (> _x 0.0)
        (set `self.isFactinRight` true)
        (else
          (set `self.isFactinRight` false)))
      (`self.AddMovementInput` (1.0 0.0 0.0) _x)
      (if (`self.isFactinRight`)
        (`self.K2_SetActorRelativeRotation` (struct))
        (else
          (`self.K2_SetActorRelativeRotation` (struct :`Yaw` 180.0))))
      (else
        (`KismetSystemLibrary.PrintString` "Move Locked")))))

(event `EnhancedInput|/Game/MyProject/C03/Input/IA_Jump01`
  (params (ActionValue :type Boolean) (ElapsedSeconds :type "Float (double-precision)") (TriggeredSeconds :type "Float (double-precision)") (InputAction :type "InputAction Object Reference" :default "/Game/MyProject/C03/Input/IA_Jump01.IA_Jump01"))
  (:`Triggered`
    (`self.Jump`)
    (`PaperFlipbookComponent.SetFlipbook` (`self.PaperFlipbook`) "/Game/U05/flipbook/fb_boy_Jump.fb_boy_Jump"))
  (:`Started`
    (`self.StopJumping` :!label _label)
    (`PaperFlipbookComponent.SetFlipbook` (`self.PaperFlipbook`) "/Game/U05/flipbook/fb_boy_Walk.fb_boy_Walk"))
  (:`Completed`
    (goto _label)))

(event `EnhancedInput|/Game/MyProject/C03/IA_Interact`
  (params (ActionValue :type Boolean) (ElapsedSeconds :type "Float (double-precision)") (TriggeredSeconds :type "Float (double-precision)") (InputAction :type "InputAction Object Reference" :default "/Game/MyProject/C03/IA_Interact.IA_Interact"))
  (:`Started`
    (bind _returnvalue (`GameplayStatics.GetActorOfClass` "/Game/MyProject/NPC_Guide/BP_NPC_Guide.BP_NPC_Guide_C"))))

(event `self.ReceiveAnyDamage`
  (params (Damage :type "Float (single-precision)") (DamageType :type "DamageType Object Reference") (InstigatedBy :type "Controller Object Reference") (DamageCauser :type "Actor Object Reference"))
  (set `self.HP` (- (`self.HP`) Damage)))

(fn `UserConstructionScript`)